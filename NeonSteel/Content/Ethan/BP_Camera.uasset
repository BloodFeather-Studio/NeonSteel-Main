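; BP_Camera is a camera actor that follows the character each tick, leading along X in its facing direction, with optionally locked height.
; WallTraceCheck line-traces both ways along the camera's forward axis from the character to flag nearby walls and store the hit.
; UpdateCamera uses that hit to scale or reverse the look-ahead and clamp X away from the wall, then smooths movement with VInterpTo.
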(event `self.ReceiveTick`
  (params (DeltaSeconds :type "Float (single-precision)"))
  (`self.UpdateCamera`))

(fn `UpdateCamera`
  (bind _walldetectouthit (`self.WallDetectOutHit`))
  (bind _character (`self.Character`))
  (bind (_walldetectouthit_bblockinghit _walldetectouthit_binitialoverlap _walldetectouthit_time _walldetectouthit_distance) (`GameplayStatics.BreakHitResult` (`self.WallDetectOutHit`)))
  (bind (_returnvalue_x _returnvalue_y _returnvalue_z) (`KismetMathLibrary.BreakVector` (`self.K2_GetActorLocation` _character)))
  (bind _returnvalue (* (`self.CameraOffset`) 1.5))
  (bind _defaultcameraheight (`/Game/Chikit/BP_ThirdPersonCharacter_Chikit.DefaultCameraHeight` _character))
  (bind _returnvalue_2 (`CapsuleComponent.GetScaledCapsuleRadius` (`Character.CapsuleComponent` (`self.Character`))))
  (bind (_returnvalue_x_2 _returnvalue_y_2 _returnvalue_z_2) (`KismetMathLibrary.BreakVector` (* (`self.GetActorForwardVector` (`self.Character`)) (`self.CameraOffset`) (`KismetMathLibrary.SelectFloat` (`KismetMathLibrary.MapRangeClamped` _walldetectouthit_distance (`self.WallDectectionRadius`) 0.0 1.0 -1.0) 1.0 (or (`self.WallDetectionRight`) (`self.WallDetectionLeft`))))))
  (bind _returnvalue_3 (- (.x (`.Location` (`GameplayStatics.BreakHitResult` _walldetectouthit))) _returnvalue _returnvalue_2))
  (bind _returnvalue_4 (+ (.x (`.Location` (`GameplayStatics.BreakHitResult` _walldetectouthit))) _returnvalue _returnvalue_2))
  (bind _returnvalue_5 (+ (`KismetMathLibrary.MakeVector` _returnvalue_x _returnvalue_y (`KismetMathLibrary.SelectFloat` (+ _defaultcameraheight (`/Game/Chikit/BP_ThirdPersonCharacter_Chikit.Camera_Z_Height` _character)) (+ _returnvalue_z _defaultcameraheight) (`/Game/Chikit/BP_ThirdPersonCharacter_Chikit.LockHeight` _character))) (`KismetMathLibrary.MakeVector` _returnvalue_x_2 0.0 _returnvalue_z_2)))
  (bind _x (.x _returnvalue_5))
  (`self.WallTraceCheck`)
  (`self.K2_SetActorLocation` (`KismetMathLibrary.VInterpTo` (`self.K2_GetActorLocation`) (`KismetMathLibrary.SelectVector` (`KismetMathLibrary.MakeVector` (`KismetMathLibrary.SelectFloat` (`KismetMathLibrary.FClamp` _x (- _returnvalue_3 50000.0) _returnvalue_3) (`KismetMathLibrary.FClamp` _x _returnvalue_4 (+ _returnvalue_4 50000.0)) (`self.WallDetectionLeft`)) (.y _returnvalue_5) (.z _returnvalue_5)) _returnvalue_5 (or (`self.WallDetectionRight`) (`self.WallDetectionLeft`))) (`GameplayStatics.GetWorldDeltaSeconds`) (`self.CameraInterpSpeed`))))

(fn `UserConstructionScript`)

(fn `WallTraceCheck`
  (bind _returnvalue (`self.GetActorForwardVector`))
  (bind _character (`self.Character`))
  (bind _returnvalue_2 (`self.K2_GetActorLocation` _character))
  (bind _returnvalue_3 (* _returnvalue (`self.WallDectectionRadius`)))
  (bind _returnvalue_4 (* (`CapsuleComponent.GetScaledCapsuleRadius` (`Character.CapsuleComponent` _character)) 0.9 _returnvalue))
  (bind (_outhit _returnvalue_5) (`KismetSystemLibrary.LineTraceSingle` :`Start` (+ _returnvalue_2 _returnvalue_4) :`End` (+ _returnvalue_2 _returnvalue_3) :`TraceChannel` "TraceTypeQuery3" :`DrawDebugType` "ForOneFrame" :`TraceColor` (struct :`G` 0.018945 :`B` 1.0 :`A` 1.0)))
  (if _returnvalue_5
    (set `self.WallDetectionLeft` true)
    (set `self.WallDetectOutHit` _outhit)
    (else
      (set `self.WallDetectionLeft` false)))
  (bind (_outhit_2 _returnvalue_6) (`KismetSystemLibrary.LineTraceSingle` :`Start` (- _returnvalue_2 _returnvalue_4) :`End` (- _returnvalue_2 _returnvalue_3) :`TraceChannel` "TraceTypeQuery4" :`DrawDebugType` "ForOneFrame" :`TraceColor` (struct :`R` 1.0 :`G` 0.911408 :`A` 1.0)))
  (if _returnvalue_6
    (set `self.WallDetectionRight` true)
    (set `self.WallDetectOutHit` _outhit_2)
    (else
      (set `self.WallDetectionRight` false)
      (if (not (or (`self.WallDetectionRight`) (`self.WallDetectionLeft`)))
        (set `self.WallDetectOutHit` (struct))))))