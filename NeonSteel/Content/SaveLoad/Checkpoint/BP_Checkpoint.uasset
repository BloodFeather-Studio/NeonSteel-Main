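; BP_Checkpoint is a checkpoint actor that saves the game when a pawn enters its collision box.
; On overlap it writes its own transform into the save game's Location variable, then requests a save through BP_GameInstance.
; A callback bound to the game-saved event only prints completion, and the save game reference it writes to is never assigned in this graph.
; Any Pawn triggers it, with a noted plan to restrict this to the player pawn.
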(event `self.Box.OnComponentBeginOverlap`
  (params (OverlappedComponent :type "PrimitiveComponent Object Reference") (OtherActor :type "Actor Object Reference") (OtherComp :type "PrimitiveComponent Object Reference") (OtherBodyIndex :type Integer) (bFromSweep :type Boolean) (SweepResult :type "HitResult Structure (by ref)"))
  ; Triggers When Pawn Passes Through Collision Box
  ;; Should Switch To Player Pawn Blueprint Later
  (cast `Pawn` OtherActor
    (:`then`
      (`KismetSystemLibrary.PrintString` "Saving Game")
      ;; Updates The Transform Variable in BP_SaveGame
      (set `/Game/SaveLoad/BP_SaveGame.Location` (`self.GetTransform`) (`self.BPSaveGameRef`))
      (bind _asbp_game_instance (cast `/Game/SaveLoad/BP_GameInstance` (`GameplayStatics.GetGameInstance`)))
      (add `/Game/SaveLoad/BP_GameInstance.GameSaved` _asbp_game_instance (delegate `Saving Completed`))
      (`/Game/SaveLoad/BP_GameInstance.RequestSave` _asbp_game_instance false))
    (:`CastFailed`
      (`KismetSystemLibrary.PrintString` "Cast Failed"))))

(event `Saving Completed`
  (params (SaveGameRef :type "/Game/SaveLoad/BP_SaveGame Object Reference"))
  ; Triggers When Pawn Passes Through Collision Box
  ;; Can Trigger Event After Saving
  (`KismetSystemLibrary.PrintString` "Saving Completed"))

(fn `UserConstructionScript`)