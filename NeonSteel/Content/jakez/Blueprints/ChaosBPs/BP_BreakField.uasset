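; BP_BreakField is a Chaos field actor that breaks destructible geometry around itself and pushes the pieces when play begins.
; It first applies external cluster strain with a linear radial falloff centered on its location.
; After a brief delay, it applies a linear force along PullDirection, using an operator field to multiply a uniform vector by a smaller, constant-strength radial mask.
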(event `self.ReceiveBeginPlay`
  (bind _returnvalue (`self.K2_GetActorLocation`))
  (`FieldSystemComponent.ApplyPhysicsField` (`self.FieldSystemComponent`) true "Field_ExternalClusterStrain" null (`RadialFalloff.SetRadialFalloff` (`self.StrainFalloff`) 500000.0 0.0 500.0 0.0 500.0 _returnvalue "Field_Falloff_Linear"))
  (`KismetSystemLibrary.Delay` 0.064)
  (`FieldSystemComponent.ApplyPhysicsField` (`self.FieldSystemComponent`) true "Field_LinearForce" null (`OperatorField.SetOperatorField` (`self.OperatorField`) 1.0 (`RadialFalloff.SetRadialFalloff` (`self.MaskFalloff`) 1.0 0.0 100.0 0.0 100.0 _returnvalue "Field_FallOff_None") (`UniformVector.SetUniformVector` (`self.UniformVector`) 50000.0 (`self.PullDirection`)) "Field_Multiply")))

(fn `UserConstructionScript`)