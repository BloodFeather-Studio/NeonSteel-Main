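; BP_Pickup is a coin pickup that increments the Pickup count on BP_ThirdPersonCharacter1.
; Overlapping Sphere with that character adds to the count and prints it on screen.
; The first CollectionCollider overlap, from any actor, activates Niagara, unhides the coin, attaches to the event's OverlappedComponent and starts an eased MoveComponentTo on the root.
; The pickup is never destroyed, and only the collection sequence is guarded by DoOnce, so counting can repeat.
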(event `self.Sphere.OnComponentBeginOverlap`
  (params (OverlappedComponent :type "PrimitiveComponent Object Reference") (OtherActor :type "Actor Object Reference") (OtherComp :type "PrimitiveComponent Object Reference") (OtherBodyIndex :type Integer) (bFromSweep :type Boolean) (SweepResult :type "HitResult Structure (by ref)"))
  (bind _asbp_third_person_character_1 (cast `/Game/PavlyBlueprints/BP_ThirdPersonCharacter1` OtherActor))
  (bind _output_get (set `/Game/PavlyBlueprints/BP_ThirdPersonCharacter1.Pickup` (+ (`/Game/PavlyBlueprints/BP_ThirdPersonCharacter1.Pickup` _asbp_third_person_character_1) 1) _asbp_third_person_character_1))
  (`KismetSystemLibrary.PrintString` (`KismetStringLibrary.Conv_IntToString` _output_get) true true (struct :`G` 0.66 :`B` 1.0 :`A` 1.0) 5.0))

(event `self.CollectionCollider.OnComponentBeginOverlap`
  (params (OverlappedComponent :type "PrimitiveComponent Object Reference") (OtherActor :type "Actor Object Reference") (OtherComp :type "PrimitiveComponent Object Reference") (OtherBodyIndex :type Integer) (bFromSweep :type Boolean) (SweepResult :type "HitResult Structure (by ref)"))
  (`/Engine/EditorBlueprintResources/StandardMacros.DoOnce` false
    (:`Completed`
      (`ActorComponent.Activate` (`self.Niagara`) false)
      (`SceneComponent.SetHiddenInGame` (`self.Coin`) false false)
      (`self.K2_AttachToComponent` OverlappedComponent "None" "KeepWorld" "KeepWorld" "KeepWorld")
      (`KismetSystemLibrary.MoveComponentTo` (`self.DefaultSceneRoot`) (0.0 0.0 0.0) (struct) true true))))

(fn `UserConstructionScript`)