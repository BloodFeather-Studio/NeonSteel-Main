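; BP_Pickup_Master is a base pickup actor that the player character collects by touching it.
; Its sphere overlap casts to BP_ThirdPersonCharacter1, then runs OnPlayerOverlap, which calls OnPickup if CanBePickedUp passes (always true here).
; OnPickup increments the character's Pickup count, prints it and destroys the actor.
; The construction script creates a dynamic material instance and sets its "Pickup" vector parameter from a variable.
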(event `self.SphereCollision.OnComponentBeginOverlap`
  (params (OverlappedComponent :type "PrimitiveComponent Object Reference") (OtherActor :type "Actor Object Reference") (OtherComp :type "PrimitiveComponent Object Reference") (OtherBodyIndex :type Integer) (bFromSweep :type Boolean) (SweepResult :type "HitResult Structure (by ref)"))
  (bind _asbp_third_person_character_1 (cast `/Game/PavlyBlueprints/BP_ThirdPersonCharacter1` OtherActor))
  (`self.OnPlayerOverlap` _asbp_third_person_character_1))

(event `OnPlayerOverlap`
  (params (Character :type "/Game/PavlyBlueprints/BP_ThirdPersonCharacter1 Object Reference"))
  (bind _canbepickedup (`self.CanBePickedUp` Character))
  (if _canbepickedup
    (`self.OnPickup` Character)))

(event `OnPickup`
  (params (Character :type "/Game/PavlyBlueprints/BP_ThirdPersonCharacter1 Object Reference"))
  (bind _output_get (set `/Game/PavlyBlueprints/BP_ThirdPersonCharacter1.Pickup` (+ (`/Game/PavlyBlueprints/BP_ThirdPersonCharacter1.Pickup` Character) 1) Character))
  (`KismetSystemLibrary.PrintString` (`KismetStringLibrary.Conv_IntToString` _output_get))
  (`self.K2_DestroyActor`))

(fn `CanBePickedUp`
  (params (Character :type "/Game/PavlyBlueprints/BP_ThirdPersonCharacter1 Object Reference"))
  (returns (CanBePickedUp :type Boolean))
  (return true))

(fn `UserConstructionScript`
  (bind _returnvalue (`PrimitiveComponent.CreateDynamicMaterialInstance` (`self.StaticMesh`) 0 "/Game/PavlyBlueprints/Pickup_Master_Material.Pickup_Master_Material" "None"))
  (bind _output_get (set `self.Material` _returnvalue))
  (`MaterialInstanceDynamic.SetVectorParameterValue` _output_get "Pickup" (`self.Pickup`)))