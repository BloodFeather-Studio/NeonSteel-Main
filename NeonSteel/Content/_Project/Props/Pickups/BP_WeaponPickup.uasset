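; Weapon pickup actor that hands its weapon to the character who interacts with it.
; Interact calls SpawnWaponPickup on that character with the weapon to spawn, the pickup location, current ammo and ammo type, then destroys the pickup.
; The reserve-ammo events and GetAmmoType are empty stubs, and the default BeginPlay, overlap and Tick events are disabled.
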(event `/Game/_Project/Interfaces/BPI_Interact.Interact`
  (params (`Character Pickiing Up` :type "/Game/ThirdPerson/Blueprints/BP_ThirdPersonCharacter Object Reference"))
  (`/Game/ThirdPerson/Blueprints/BP_ThirdPersonCharacter.Spawn Wapon/Pickup` `Character Pickiing Up` (`self.WeaponToSpawn`) (`self.K2_GetActorLocation`) (`self.Current Ammo`) (`self.Ammos`))
  (`self.K2_DestroyActor`))

(event `/Game/_Project/Interfaces/BPI_WeaponPickUp.Take Reserve Ammo`
  (params (`Ammo Taken` :type Integer)))

(event `/Game/_Project/Interfaces/BPI_WeaponPickUp.Update Current Reserve Ammo`)

(fn `Get Ammo Type`
  (returns (`Ammo Type` :type "/Game/_Project/Props/Weapons/Struct_Ammo Structure"))
  (return))

(fn `UserConstructionScript`
  (`parent.UserConstructionScript`))