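; Projectile Blueprint, apparently a master class, that damages what it hits and breaks Chaos destructibles.
; On sphere hit it sends an ApplyDamage message to the other actor, then destroys itself.
; It also spawns a short-lived, triggered FS_MasterField at that actor's origin rather than the impact point to drive destruction.
; Older radial force, radial damage and impact effect logic, including NewFunction, remains but never runs.
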(event `self.ReceiveHit`
  (params (MyComp :type "PrimitiveComponent Object Reference") (Other :type "Actor Object Reference") (OtherComp :type "PrimitiveComponent Object Reference") (bSelfMoved :type Boolean) (HitLocation :type "Vector Structure") (HitNormal :type "Vector Structure") (NormalImpulse :type "Vector Structure") (Hit :type "HitResult Structure (by ref)")))

(event `self.Sphere.OnComponentHit`
  (params (HitComponent :type "PrimitiveComponent Object Reference") (OtherActor :type "Actor Object Reference") (OtherComp :type "PrimitiveComponent Object Reference") (NormalImpulse :type "Vector Structure") (Hit :type "HitResult Structure (by ref)"))
  (bind (_returnvalue_location _returnvalue_rotation) (`KismetMathLibrary.BreakTransform` (`self.GetTransform` OtherActor)))
  (message `/Game/_Project/Props/BLI/BLI_Damagable.ApplyDamage` OtherActor)
  (bind _returnvalue (`|SpawnActorFromClass` "/Engine/EditorResources/FieldNodes/FS_MasterField.FS_MasterField_C" (`KismetMathLibrary.MakeTransform` _returnvalue_location _returnvalue_rotation (* (1.0 1.0 1.0) 2.0)) "Undefined" "MultiplyWithRoot" null null))
  (bind _output_get (set `self.Chaos` _returnvalue))
  (set `/Engine/EditorResources/FieldNodes/FS_MasterField.Radial Magnitude` 100.0 _output_get)
  (`self.SetLifeSpan` _output_get 0.2)
  (set `/Engine/EditorResources/FieldNodes/FS_MasterField.ActivationType` "NewEnumerator4" _output_get)
  (`/Engine/EditorResources/FieldNodes/FS_MasterField.CE_Trigger` _output_get)
  (`self.K2_DestroyActor`))

(fn `NewFunction`
  (params (Hit :type "HitResult Structure (by ref)"))
  (bind (_bblockinghit _binitialoverlap _time _distance _location _impactpoint _normal) (`GameplayStatics.BreakHitResult` Hit))
  (`PrimitiveComponent.SetCollisionEnabled` (`self.Sphere`) "NoCollision")
  (`RadialForceComponent.FireImpulse` (`self.RadialForce`))
  (`GameplayStatics.SpawnEmitterAtLocation` "/Game/MilitaryWeapDark/FX/P_Impact_Metal_Small_01.P_Impact_Metal_Small_01" _location (`KismetMathLibrary.MakeRotFromX` _normal))
  (`GameplayStatics.PlaySoundAtLocation` "/Engine/VREditor/Sounds/UI/Laser_Pull.Laser_Pull" _location (struct) 1.0 1.0 0.0 null null null null)
  (`self.K2_DestroyActor`))

(fn `UserConstructionScript`)