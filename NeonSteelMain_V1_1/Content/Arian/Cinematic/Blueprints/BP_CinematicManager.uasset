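; BP_CinematicManager plays the opening cinematic and moves the game to the main map when the video ends or is skipped.
; On BeginPlay it shows the cinematic widget with UI-only focus and a hidden cursor, then opens the media source, playing once loaded.
; A guarded transition closes the media, swaps in a loading screen and opens the map after a short delay.
; The audio volume logic is unconnected.
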(event `self.ReceiveBeginPlay`
  (bind _returnvalue (`GameplayStatics.GetPlayerController` 0))
  (set `PlayerController.bShowMouseCursor` false _returnvalue)
  (`WidgetBlueprintLibrary.SetInputMode_GameOnly` _returnvalue)
  (`MediaPlayer.Close` (`self.Opening Media Player`))
  (add `MediaPlayer.OnMediaOpened` (`self.Opening Media Player`) (delegate `HandleMediaOpened`))
  (add `MediaPlayer.OnEndReached` (`self.Opening Media Player`) (delegate `HandleCinematicEnded`))
  (bind _returnvalue_2 (`|CreateWidget` (`self.Cinematic Widget Class`) (`GameplayStatics.GetPlayerController` 0)))
  (bind _output_get (set `self.Cinematic Widget Ref` _returnvalue_2))
  (add `/Game/Arian/Cinematic/Widgets/WBP_CinematicPlayer.OnSkipCompleted` _output_get (delegate `HandleSkipCompleted`))
  (`UserWidget.AddToViewport` _output_get 0)
  (`KismetSystemLibrary.Delay` 0.0)
  (bind _returnvalue_3 (`GameplayStatics.GetPlayerController` 0))
  (set `PlayerController.bShowMouseCursor` false _returnvalue_3)
  (`WidgetBlueprintLibrary.SetInputMode_UIOnlyEx` _returnvalue_3 (`self.Cinematic Widget Ref`))
  (`Widget.SetUserFocus` (`self.Cinematic Widget Ref`) _returnvalue_3)
  (`Widget.SetKeyboardFocus` (`self.Cinematic Widget Ref`))
  (bind _returnvalue_4 (`MediaPlayer.OpenSource` (`self.Opening Media Player`) (`self.Opening Media Source`)))
  (if (not _returnvalue_4)
    (`KismetSystemLibrary.PrintString` "Failed to open OpeningCinematic")))

(event `HandleMediaOpened`
  (params (OpenedUrl :type String))
  (`MediaPlayer.Play` (`self.Opening Media Player`)))

(event `HandleSkipCompleted`
  (`self.BeginTransitionToMainMap`))

(event `HandleCinematicEnded`
  (`self.BeginTransitionToMainMap`))

(event `BeginTransitionToMainMap`
  (if (not (`self.Is Transitioning To Main Map`))
    (set `self.Is Transitioning To Main Map` true)
    (`MediaPlayer.Close` (`self.Opening Media Player`))
    (`/Engine/EditorBlueprintResources/StandardMacros.IsValid` (`self.Cinematic Widget Ref`)
      (:`Is Valid`
        (`Widget.RemoveFromParent` (`self.Cinematic Widget Ref`))
        (bind _returnvalue (`GameplayStatics.GetPlayerController` 0))
        (bind _returnvalue_2 (`|CreateWidget` (`self.Loading Screen Widget Class`) _returnvalue))
        (bind _output_get (set `self.Loading Screen Widget Ref` _returnvalue_2))
        (`UserWidget.AddToViewport` _output_get 0)
        (`/Game/Arian/Cinematic/Widgets/WBP_CinematicPlayer.ResetInputForGameplay` (`self.Cinematic Widget Ref`))
        (`KismetSystemLibrary.Delay` 1.2)
        (`GameplayStatics.OpenLevel` (`self.Main Map Name`))))))

(fn `UserConstructionScript`)