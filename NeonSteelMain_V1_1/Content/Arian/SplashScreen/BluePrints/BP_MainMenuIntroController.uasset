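; Controller actor that plays the main menu intro level sequence and signals when it has finished.
; BeginPlay caches the player controller and binds to the sequence player's finished event, while PlayMainMenuIntro starts playback only once.
; On finish, it switches the view target to the final menu camera if valid, then calls OnMainMenuIntroFinished.
; A missing sequence actor on play still fires that notification, so the menu flow can continue.
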(event `self.ReceiveBeginPlay`
  (`/Engine/EditorBlueprintResources/StandardMacros.IsValid` (`self.MainMenuIntroSequenceActor`)
    (:`Is Valid`
      (bind _returnvalue (`GameplayStatics.GetPlayerController` 0))
      (set `self.PlayerControllerRef` _returnvalue)
      (add `MovieSceneSequencePlayer.OnFinished` (`LevelSequenceActor.SequencePlayer` (`self.MainMenuIntroSequenceActor`)) (delegate `HandleIntroSequenceFinished`)))
    (:`Is Not Valid`
      (`KismetSystemLibrary.PrintString` "BP_MainMenuIntroController Invalid"))))

(event `HandleIntroSequenceFinished`
  (`/Engine/EditorBlueprintResources/StandardMacros.IsValid` (`self.FinalMenuCamera`)
    (:`Is Valid`
      (`PlayerController.SetViewTargetWithBlend` (`self.PlayerControllerRef`) (`self.FinalMenuCamera`) 0.0 "VTBlend_Linear" 0.0 false)
      (`self.OnMainMenuIntroFinished`))
    (:`Is Not Valid`
      (`self.OnMainMenuIntroFinished`))))

(fn `PlayMainMenuIntro`
  (if (not (`self.bIntroAlreadyPlayed`))
    (set `self.bIntroAlreadyPlayed` true)
    (`/Engine/EditorBlueprintResources/StandardMacros.IsValid` (`self.MainMenuIntroSequenceActor`)
      (:`Is Valid`
        (`MovieSceneSequencePlayer.Play` (`LevelSequenceActor.SequencePlayer` (`self.MainMenuIntroSequenceActor`))))
      (:`Is Not Valid`
        (`KismetSystemLibrary.PrintString` "Cannot play main menu intro \nSequence actor is missing")
        (`self.OnMainMenuIntroFinished`)))))

(fn `UserConstructionScript`)