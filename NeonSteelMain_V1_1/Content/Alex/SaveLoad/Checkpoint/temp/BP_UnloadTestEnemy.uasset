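; BP_UnloadTestEnemy is a test enemy that decides at level start whether to remove itself based on checkpoint save data.
; On BeginPlay it reads its killed flag by EnemyID from the game instance's SaveGame.
; It destroys itself only if killed and its X position is at or behind the saved checkpoint's X, otherwise printing debug messages.
; Death logic that would set the killed flag exists but is unconnected.
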(event `self.ReceiveBeginPlay`
  ; Enemy BeginPlay Logic to Determine if Enemy Should be Destroyed or Not
  (bind _asbp_game_instance (cast `/Game/Alex/SaveLoad/BP_GameInstance` (`GameplayStatics.GetGameInstance`))
    (:`then`
      (bind _output_get (set `self.As BP Game Instance` _asbp_game_instance))
      ;; Checks to See if Enemy Has Been Killed
      (if (`|GetArrayItem` (`/Game/Alex/SaveLoad/BP_SaveGame.CurrentEnemyStates` (`/Game/Alex/SaveLoad/BP_GameInstance.SaveGameRef` _output_get)) (`self.EnemyID`))
        ;; Checks to See if Enemy is Behind Current Checkpoint
        (if (>= (.x (.location (`/Game/Alex/SaveLoad/BP_SaveGame.Location` (`/Game/Alex/SaveLoad/BP_GameInstance.SaveGameRef` (`self.As BP Game Instance`))))) (.x (.location (`self.GetTransform`))))
          (`self.K2_DestroyActor`)
          (else
            (`KismetSystemLibrary.PrintString` "Enemy is Ahead of Checkpoint")))
        (else
          (`KismetSystemLibrary.PrintString` "Enemy is Still Alive"))))
    (:`CastFailed`
      (`KismetSystemLibrary.PrintString` "Cast Failed on UnloadTestEnemy"))))

(fn `UserConstructionScript`)