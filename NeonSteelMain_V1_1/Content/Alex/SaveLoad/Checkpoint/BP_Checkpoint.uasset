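; Checkpoint actor that saves the game when BP_Player overlaps its box.
; It writes its own transform and the player's total ammo and current neon into the SaveGameRef held by BP_GameInstance.
; It then binds a completion callback and requests a save through the game instance, printing debug strings along the way.
; A player-health save branch with a zero-health fallback is present but disconnected.
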(event `self.Box.OnComponentBeginOverlap`
  (params (OverlappedComponent :type "PrimitiveComponent Object Reference") (OtherActor :type "Actor Object Reference") (OtherComp :type "PrimitiveComponent Object Reference") (OtherBodyIndex :type Integer) (bFromSweep :type Boolean) (SweepResult :type "HitResult Structure (by ref)"))
  ; Triggers When Pawn Passes Through Collision Box
  (bind _asbp_player (cast `/Game/Variant_SideScroller/Blueprints/Player/BP_Player` OtherActor)
    (:`then`
      (`KismetSystemLibrary.PrintString` "Saving Game")
      (bind _asbp_game_instance (cast `/Game/Alex/SaveLoad/BP_GameInstance` (`GameplayStatics.GetGameInstance`))
        (:`then`
          (bind _savegameref (`/Game/Alex/SaveLoad/BP_GameInstance.SaveGameRef` _asbp_game_instance))
          ;; Updates The Transform Variable in BP_SaveGame
          (bind _output_get (set `/Game/Alex/SaveLoad/BP_SaveGame.Location` (`self.GetTransform`) _savegameref))
          (`KismetSystemLibrary.PrintString` (`KismetStringLibrary.Conv_TransformToString` _output_get))
          ;; Updates PlayerBullets from BP_Player  for BP_SaveGame
          (bind _output_get_2 (set `/Game/Alex/SaveLoad/BP_SaveGame.PlayerBullets` (`/Game/Variant_SideScroller/Blueprints/Player/BP_Player.TotalAmmo` _asbp_player) _savegameref))
          (`KismetSystemLibrary.PrintString` (`KismetStringLibrary.Conv_IntToString` _output_get_2))
          ;; Updates PlayerNeon from BP_Player  for BP_SaveGame
          (bind _output_get_3 (set `/Game/Alex/SaveLoad/BP_SaveGame.PlayerNeon` (`/Game/Variant_SideScroller/Blueprints/Player/BP_Player.NeonCurrent` _asbp_player) _savegameref))
          (`KismetSystemLibrary.PrintString` (`KismetStringLibrary.Conv_DoubleToString` _output_get_3))
          (add `/Game/Alex/SaveLoad/BP_GameInstance.GameSaved` _asbp_game_instance (delegate `Saving Completed`))
          (`/Game/Alex/SaveLoad/BP_GameInstance.RequestSave` _asbp_game_instance false))
        (:`CastFailed`
          (`KismetSystemLibrary.PrintString` "Cast Failed"))))
    (:`CastFailed`
      (`KismetSystemLibrary.PrintString` "Cast Failed"))))

(event `Saving Completed`
  (params (SaveGameRef :type "/Game/Alex/SaveLoad/BP_SaveGame Object Reference"))
  ; Triggers When Pawn Passes Through Collision Box
  ;; Can Trigger Event After Saving
  (`KismetSystemLibrary.PrintString` "Saving Completed"))

(fn `UserConstructionScript`)