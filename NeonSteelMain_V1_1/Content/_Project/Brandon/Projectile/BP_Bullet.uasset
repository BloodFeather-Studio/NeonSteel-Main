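; BP_Bullet is a projectile actor that damages what it hits and then destroys itself.
; A sphere component hit applies damage to any valid actor and spawns a short-lived FS_MasterField at that actor's transform, triggering a Chaos field.
; The actor Hit event sends a randomly selected damage amount to actors tagged Enemy through ApplyDamageMessage, and destroys the bullet whatever it hits.
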(event `self.Sphere.OnComponentHit`
  (params (HitComponent :type "PrimitiveComponent Object Reference") (OtherActor :type "Actor Object Reference") (OtherComp :type "PrimitiveComponent Object Reference") (NormalImpulse :type "Vector Structure") (Hit :type "HitResult Structure (by ref)"))
  (bind (_returnvalue_location _returnvalue_rotation) (`KismetMathLibrary.BreakTransform` (`self.GetTransform` OtherActor)))
  (`/Engine/EditorBlueprintResources/StandardMacros.IsValid` OtherActor
    (:`Is Valid`
      (if true
        (`GameplayStatics.ApplyDamage` OtherActor)
        (bind _returnvalue (`|SpawnActorFromClass` "/Engine/EditorResources/FieldNodes/FS_MasterField.FS_MasterField_C" (`KismetMathLibrary.MakeTransform` _returnvalue_location _returnvalue_rotation (* (1.0 1.0 1.0) 1.0)) "Undefined" "MultiplyWithRoot" null null))
        (bind _output_get (set `self.Chaos` _returnvalue))
        (set `/Engine/EditorResources/FieldNodes/FS_MasterField.Radial Magnitude` 1.0 _output_get)
        (`self.SetLifeSpan` _returnvalue 0.2)
        (set `/Engine/EditorResources/FieldNodes/FS_MasterField.ActivationType` "NewEnumerator4" _returnvalue)
        (`/Engine/EditorResources/FieldNodes/FS_MasterField.CE_Trigger` _returnvalue)
        (`self.K2_DestroyActor`)))))

(event `self.ReceiveHit`
  (params (MyComp :type "PrimitiveComponent Object Reference") (Other :type "Actor Object Reference") (OtherComp :type "PrimitiveComponent Object Reference") (bSelfMoved :type Boolean) (HitLocation :type "Vector Structure") (HitNormal :type "Vector Structure") (NormalImpulse :type "Vector Structure") (Hit :type "HitResult Structure (by ref)"))
  (if (`self.ActorHasTag` Other "Enemy")
    (message `/Game/Ethan/Blueprints/BPI_Damageable.Apply Damage` Other (select `int` (`KismetMathLibrary.RandomInteger` 3) :`0` 10.0 :`1` 25.0 :`2` 85.0 :`3` 35.0 :!type "Float (single-precision)") self (0.0 0.0 0.0) (0.0 0.0 0.0))
    (`self.K2_DestroyActor`)
    (else
      (`self.K2_DestroyActor`))))

(fn `UserConstructionScript`)