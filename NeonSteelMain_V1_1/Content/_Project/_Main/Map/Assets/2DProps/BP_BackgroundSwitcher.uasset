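; BP_BackgroundSwitcher is a one-shot trigger actor that changes the sky background when the player character overlaps it.
; On BeginPlay it caches the B_SkyTexture actor found in the level.
; Player overlap passes the switcher's SkyTexture to that actor's ChangeSkyTexture.
; When the player leaves the overlap, it sets Disabled, so later entries no longer switch the sky.
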(event `self.ReceiveBeginPlay`
  (bind _returnvalue (`GameplayStatics.GetActorOfClass` "/Game/_Project/_Main/Map/Assets/2DProps/B_SkyTexture.B_SkyTexture_C"))
  (set `self.Sky Mesh` _returnvalue))

(event `self.ReceiveActorBeginOverlap`
  (params (OtherActor :type "Actor Object Reference"))
  (if (and (== OtherActor (`GameplayStatics.GetPlayerCharacter` 0)) (not (`self.Disabled`)))
    (`/Game/_Project/_Main/Map/Assets/2DProps/B_SkyTexture.Change Sky Texture` (`self.Sky Mesh`) (`self.Sky Texture`))))

(event `self.ReceiveActorEndOverlap`
  (params (OtherActor :type "Actor Object Reference"))
  (if (== OtherActor (`GameplayStatics.GetPlayerCharacter` 0))
    (set `self.Disabled` true)))

(fn `UserConstructionScript`)