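; BP_AudioZone is a placed zone actor that switches the game's music zone when the player is inside it.
; When BP_Player begins overlapping the Area component, it passes its TargetZone to UpdateMusicZone on BP_GameInstance.
; A half-second delayed check after BeginPlay makes the same call if the player already overlaps the actor.
; Leaving the zone triggers nothing.
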(event `self.ReceiveBeginPlay`
  (`KismetSystemLibrary.Delay` 0.5)
  (if (> (`KismetArrayLibrary.Array_Length` (`self.GetOverlappingActors` "/Game/Variant_SideScroller/Blueprints/Player/BP_Player.BP_Player_C")) 0)
    (bind _asbp_game_instance (cast `/Game/Alex/SaveLoad/BP_GameInstance` (`GameplayStatics.GetGameInstance`)))
    (`/Game/Alex/SaveLoad/BP_GameInstance.UpdateMusicZone` _asbp_game_instance (`self.TargetZone`))))

(event `self.Area.OnComponentBeginOverlap`
  (params (OverlappedComponent :type "PrimitiveComponent Object Reference") (OtherActor :type "Actor Object Reference") (OtherComp :type "PrimitiveComponent Object Reference") (OtherBodyIndex :type Integer) (bFromSweep :type Boolean) (SweepResult :type "HitResult Structure (by ref)"))
  (cast `/Game/Variant_SideScroller/Blueprints/Player/BP_Player` OtherActor)
  (bind _asbp_game_instance (cast `/Game/Alex/SaveLoad/BP_GameInstance` (`GameplayStatics.GetGameInstance`)))
  (`/Game/Alex/SaveLoad/BP_GameInstance.UpdateMusicZone` _asbp_game_instance (`self.TargetZone`)))

(fn `UserConstructionScript`)