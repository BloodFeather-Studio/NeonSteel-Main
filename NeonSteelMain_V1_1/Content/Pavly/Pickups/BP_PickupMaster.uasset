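; BP_PickupMaster is a pickup actor that magnetically flies to a target and delivers its PickupData, likely as a base for other pickups.
; StartAttract stores the target and enables Tick, which interpolates toward the component and spawns an attached magnet sound every frame.
; Within CollectDistance, it passes data through BPI_PickupReciever if the target accepts.
; It destroys itself even when refused, or if the target component becomes invalid.
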(event `self.ReceiveTick`
  (params (DeltaSeconds :type "Float (single-precision)"))
  (bind _targetcomponent (`self.TargetComponent`))
  ; For every frame, set Attracting? to true which takes the Input object which is the target component (Player Magnetic Sphere), the program determines the location of the player and the location of the pickup. Once those aspects of teh program are determined, then the Move and Collect Check functions are initialized.
  (bind _output_get (set `self.Attracting` (`self.Attracting`)))
  (if _output_get
    (`/Engine/EditorBlueprintResources/StandardMacros.IsValid` _targetcomponent
      (:`Is Valid`
        (set `self.TargetLocation` (`SceneComponent.K2_GetComponentLocation` _targetcomponent))
        (set `self.CurrentLocation` (`self.K2_GetActorLocation`))
        (`GameplayStatics.SpawnSoundAttached` "/Game/Audio/METASOUNDS/Environment/Pickups/MS_Pickup_Magnet.MS_Pickup_Magnet" (`self.StaticMesh`) "None" (0.0 0.0 0.0) (struct) "KeepRelativeOffset" false 1.0 1.0 0.0 null null)
        (`self.Move`)
        (`self.CollectCheck`))
      (:`Is Not Valid`
        (set `self.Attracting` false)
        (`self.SetActorTickEnabled` false)
        (`self.K2_DestroyActor`)))))

(fn `CanRecievePickups`
  (params (PickupData :type "/Game/Pavly/Structs/ST_PickupData Structure"))
  (returns (CanRecieve :type Boolean))
  (return false))

(fn `CollectCheck`
  ; This function takes the new location of the Pickup and the target location which is the location of the player and it turns the two distances into a return value that is compared to the collection distance that results in the comparison of the two values that determines whether it goes to the next function (Finish Collect) or not.
  (if (<= (`KismetMathLibrary.Vector_Distance` (`self.NewLocation`) (`self.TargetLocation`)) (`self.CollectDistance`))
    (`self.FinishCollect`)))

(fn `FinishCollect`
  (bind _targetactor (`self.TargetActor`))
  (bind _pickupdata (`self.PickupData`))
  ; This function finishes the collecting of the pickup
  (`KismetSystemLibrary.PrintString` "FinishCollect TargetActor" true true (struct :`G` 0.66 :`B` 1.0 :`A` 1.0) 5.0)
  (`self.SetActorTickEnabled` false)
  (set `self.Attracting` false)
  (if (`KismetSystemLibrary.DoesImplementInterface` _targetactor "/Game/Pavly/Interface/BPI_PickupReciever.BPI_PickupReciever_C")
    (bind _canrecieve (message `/Game/Pavly/Interface/BPI_PickupReciever.CanRecievePickups` _targetactor _pickupdata))
    (if _canrecieve
      (message `/Game/Pavly/Interface/BPI_PickupReciever.RecievePickups` _targetactor _pickupdata self)
      (`self.K2_DestroyActor`)
      (else
        (`self.K2_DestroyActor`)))
    (else
      (`KismetSystemLibrary.PrintString` "TargetActor was not received" true true (struct :`G` 0.66 :`B` 1.0 :`A` 1.0) 5.0)
      (`self.K2_DestroyActor`))))

(fn `Move`
  ; Determines current location of pickup and the location of the player then returns the value of the new location for the pickup to travel to. It also determines the travel speed of the pickup.
  (bind _output_get (set `self.NewLocation` (`KismetMathLibrary.VInterpTo` (`self.CurrentLocation`) (`self.TargetLocation`) (`GameplayStatics.GetWorldDeltaSeconds`) (`self.MagnetInterpSpeed`))))
  (`self.K2_SetActorLocation` _output_get))

(fn `StartAttract`
  (params (inTargetActor :type "Actor Object Reference") (inTargetComponent :type "SceneComponent Object Reference"))
  (returns (TargetActor :type "Actor Object Reference") (TargetComponent :type "SceneComponent Object Reference"))
  ; This function determines the Target Actor which is the Player and the Target Component is the Scene component in the Pickup then it checks the condition if they are attracting. If they are attracting then it returns the assigned Target Actor (Player) and Target Component (Pickup). If it returns false, then it assigns the player to target actor and pickup to target component and the assigns them to attracting.
  (if (not (`self.Attracting`))
    (bind _output_get (set `self.TargetActor` inTargetActor))
    (`KismetSystemLibrary.PrintString` "StartAttract set TargetActor" true true (struct :`G` 0.66 :`B` 1.0 :`A` 1.0) 5.0)
    (bind _output_get_2 (set `self.TargetComponent` inTargetComponent))
    (set `self.Attracting` true)
    (`self.SetActorTickEnabled` true))
  (return _output_get _output_get_2))

(fn `UserConstructionScript`)