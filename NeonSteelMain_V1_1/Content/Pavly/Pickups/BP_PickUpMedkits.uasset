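; Medkit pickup that homes in on the player's PickupSocket once a BP_Player overlaps its sphere.
; Overlap enables Tick, which interpolates the actor toward the socket until it is within collect distance, then finishes collection.
; The pickup passes itself as target actor, so its own receiver interface is queried; CanRecievePickups returns false, so it is destroyed without delivering its data.
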(event `self.ReceiveTick`
  (params (DeltaSeconds :type "Float (single-precision)"))
  ; For every frame, set Attracting? to true which takes the Input object which is the target component (Player Magnetic Sphere), the program determines the location of the player and the location of the pickup. Once those aspects of teh program are determined, then the Move and Collect Check functions are initialized.
  (bind _output_get (set `self.AttractingChild` (`self.AttractingChild`)))
  (if _output_get
    (`/Engine/EditorBlueprintResources/StandardMacros.IsValid` (`self.TargetComponentChild`)
      (:`Is Valid`
        (set `self.TargetLocationChild` (`SceneComponent.K2_GetComponentLocation` (`self.TargetComponentChild`)))
        (set `self.CurrentLocationChild` (`self.K2_GetActorLocation`))
        (`self.MoveChild`)
        (`self.CollectCheckChild`))
      (:`Is Not Valid`
        (set `self.AttractingChild` false)
        (`self.SetActorTickEnabled` false)
        (`self.K2_DestroyActor`)))))

(event `self.Sphere.OnComponentBeginOverlap`
  (params (OverlappedComponent :type "PrimitiveComponent Object Reference") (OtherActor :type "Actor Object Reference") (OtherComp :type "PrimitiveComponent Object Reference") (OtherBodyIndex :type Integer) (bFromSweep :type Boolean) (SweepResult :type "HitResult Structure (by ref)"))
  (bind _asbp_player (cast `/Game/Variant_SideScroller/Blueprints/Player/BP_Player` OtherActor))
  (`self.StartAttractChild` self (`/Game/Variant_SideScroller/Blueprints/Player/BP_Player.PickupSocket` _asbp_player)))

(event `self.RecievePickups`
  (params (PickupData :type "/Game/Pavly/Structs/ST_PickupData Structure") (PickupActor :type "Actor Object Reference"))
  (switch `/Game/Pavly/Enums/E_PickupType` (`.Type_15_ED94AC604F79BAF7D0ABE7A935D7AB30` (break `/Game/Pavly/Structs/ST_PickupData` PickupData))
    (:`NewEnumerator2`
      (`KismetSystemLibrary.PrintString` "Medkit Picked up"))))

(fn `CanRecievePickups`
  (params (PickupData :type "/Game/Pavly/Structs/ST_PickupData Structure"))
  (returns (CanRecieve :type Boolean))
  (return false))

(fn `CollectCheckChild`
  ; This function takes the new location of the Pickup and the target location which is the location of the player and it turns the two distances into a return value that is compared to the collection distance that results in the comparison of the two values that determines whether it goes to the next function (Finish Collect) or not.
  (if (<= (`KismetMathLibrary.Vector_Distance` (`self.NewLocationChild`) (`self.TargetLocationChild`)) (`self.CollectDistanceChild`))
    (`self.FinishCollectChild`)))

(fn `FinishCollectChild`
  (bind _pickupdatachild (`self.PickupDataChild`))
  (bind _targetactorchild (`self.TargetActorChild`))
  ; This function finishes the collecting of the pickup
  (`self.SetActorTickEnabled` false)
  (set `self.AttractingChild` false)
  (if (`KismetSystemLibrary.DoesImplementInterface` _targetactorchild "/Game/Pavly/Interface/BPI_PickupReciever.BPI_PickupReciever_C")
    (bind _canrecieve (message `/Game/Pavly/Interface/BPI_PickupReciever.CanRecievePickups` _targetactorchild _pickupdatachild))
    (if _canrecieve
      (message `/Game/Pavly/Interface/BPI_PickupReciever.RecievePickups` _targetactorchild _pickupdatachild self)
      (`self.K2_DestroyActor`)
      (else
        (`self.K2_DestroyActor`)))
    (else
      (`KismetSystemLibrary.PrintString` "TargetActor was not received")
      (`self.K2_DestroyActor`))))

(fn `MoveChild`
  ; Determines current location of pickup and the location of the player then returns the value of the new location for the pickup to travel to. It also determines the travel speed of the pickup.
  (bind _output_get (set `self.NewLocationChild` (`KismetMathLibrary.VInterpTo` (`self.CurrentLocationChild`) (`self.TargetLocationChild`) (`GameplayStatics.GetWorldDeltaSeconds`) (`self.MagnetInterpSpeedChild`))))
  (`self.K2_SetActorLocation` _output_get))

(fn `StartAttractChild`
  (params (inTargetActor :type "Actor Object Reference") (inTargetComponent :type "SceneComponent Object Reference"))
  (returns (TargetActor :type "Actor Object Reference") (TargetComponent :type "SceneComponent Object Reference"))
  ; This function determines the Target Actor which is the Player and the Target Component is the Scene component in the Pickup then it checks the condition if they are attracting. If they are attracting then it returns the assigned Target Actor (Player) and Target Component (Pickup). If it returns false, then it assigns the player to target actor and pickup to target component and the assigns them to attracting.
  (if (not (`self.AttractingChild`))
    (bind _output_get (set `self.TargetActorChild` inTargetActor))
    (bind _output_get_2 (set `self.TargetComponentChild` inTargetComponent))
    (set `self.AttractingChild` true)
    (`self.SetActorTickEnabled` true))
  (return _output_get _output_get_2))

(fn `UserConstructionScript`)