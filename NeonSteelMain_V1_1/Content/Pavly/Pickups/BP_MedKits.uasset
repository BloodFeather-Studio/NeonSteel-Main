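; BP_MedKits is a med kit pickup that gets magnetically attracted to the player.
; When BP_Player overlaps its Sphere, it plays a magnet sound attached to its StaticMesh and calls StartAttract toward the player's PickupSocket component, passing itself as the target actor.
; The graph holds no healing or collection logic, and its BeginPlay, Tick and actor overlap events are disabled.
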(event `self.Sphere.OnComponentBeginOverlap`
  (params (OverlappedComponent :type "PrimitiveComponent Object Reference") (OtherActor :type "Actor Object Reference") (OtherComp :type "PrimitiveComponent Object Reference") (OtherBodyIndex :type Integer) (bFromSweep :type Boolean) (SweepResult :type "HitResult Structure (by ref)"))
  (bind _asbp_player (cast `/Game/Variant_SideScroller/Blueprints/Player/BP_Player` OtherActor))
  (`GameplayStatics.SpawnSoundAttached` "/Game/Audio/METASOUNDS/Environment/Pickups/MS_Pickup_Magnet.MS_Pickup_Magnet" (`self.StaticMesh`) "None" (0.0 0.0 0.0) (struct) "KeepRelativeOffset" false 1.0 1.0 0.0 null null)
  (`self.StartAttract` self (`/Game/Variant_SideScroller/Blueprints/Player/BP_Player.PickupSocket` _asbp_player)))

(fn `UserConstructionScript`
  (`parent.UserConstructionScript`))