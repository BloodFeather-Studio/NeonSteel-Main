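; Actor component that spawns run-dust effects under a moving Character.
; A looping timer checks horizontal speed against a threshold, then line-traces downward to find ground.
; On a hit, it spawns a BP_RunDustVFX with the dust material near the impact point, offset and rotated relative to the owner.
; The spawn's X scale mirrors based on the sign of world X velocity, flipping the effect with travel direction.
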(event `self.ReceiveBeginPlay`
  (`KismetSystemLibrary.K2_SetTimerDelegate` (delegate `Try Spawn Dust`) (`self.Spawn Interval`) true))

(event `Try Spawn Dust`
  (bind _returnvalue (`self.GetOwner`))
  (bind _returnvalue_2 (`self.GetOwner`))
  (bind _returnvalue_3 (`Actor.K2_GetActorLocation` _returnvalue))
  (cast `Character` _returnvalue)
  (if (> (`KismetMathLibrary.VSizeXY` (`Actor.GetVelocity` _returnvalue)) (`self.Speed Threshold`))
    (bind (_outhit _returnvalue_4) (`KismetSystemLibrary.LineTraceSingle` (+ _returnvalue_3 (0.0 0.0 20.0)) (- _returnvalue_3 (`KismetMathLibrary.MakeVector` 0.0 0.0 (`KismetMathLibrary.Conv_IntToDouble` (`self.Ground Trace Distance`)))) "TraceTypeQuery1"))
    (if _returnvalue_4
      (`|SpawnActorFromClass` "/Game/Brandon/VFX/RunDust-VFX/BP_RunDustVFX.BP_RunDustVFX_C" (`KismetMathLibrary.MakeTransform` (+ (+ (`.ImpactPoint` (`GameplayStatics.BreakHitResult` _outhit)) (`Actor.GetActorForwardVector` _returnvalue_2)) (20.0 0.0 30.0)) (`KismetMathLibrary.ComposeRotators` (`Actor.K2_GetActorRotation` _returnvalue_2) (`KismetMathLibrary.MakeRotator` 0.0 90.0 90.0)) (`KismetMathLibrary.SelectVector` (-2.0 2.0 2.0) (2.0 2.0 2.0) (< (.x (`Actor.GetVelocity` _returnvalue_2)) 0.0))) "Undefined" "MultiplyWithRoot" null "/Game/Brandon/VFX/RunDust-VFX/M_RunDust_Inst.M_RunDust_Inst" null))))