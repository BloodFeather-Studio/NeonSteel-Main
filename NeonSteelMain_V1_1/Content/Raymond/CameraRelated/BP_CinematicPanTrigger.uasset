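; A trigger volume that plays a one-time cinematic camera pan when the player walks into it.
; On box overlap with BP_Player, it disables movement input and tells the BP_SideScrollingCameraManager to pan using per-instance offsets and zoom.
; A WalkedThru flag prevents repeat triggering, and a fixed delay restores player movement afterwards without checking whether the pan has finished.
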(event `self.ReceiveBeginPlay`)

(event `self.Box.OnComponentBeginOverlap`
  (params (OverlappedComponent :type "PrimitiveComponent Object Reference") (OtherActor :type "Actor Object Reference") (OtherComp :type "PrimitiveComponent Object Reference") (OtherBodyIndex :type Integer) (bFromSweep :type Boolean) (SweepResult :type "HitResult Structure (by ref)"))
  (bind _asbp_player (cast `/Game/Variant_SideScroller/Blueprints/Player/BP_Player` OtherActor))
  (if (not (`self.WalkedThru`))
    (set `/Game/Variant_SideScroller/Blueprints/Player/BP_Player.MovementInput` false _asbp_player)
    (bind _asbp_side_scrolling_camera_manager (cast `/Game/Variant_SideScroller/Blueprints/BP_SideScrollingCameraManager` (`GameplayStatics.GetPlayerCameraManager` 0)))
    (`/Game/Variant_SideScroller/Blueprints/BP_SideScrollingCameraManager.EnableCameraPan` _asbp_side_scrolling_camera_manager (`self.Custom Pan X`) (+ (`self.CusomZoom`) 1000.0) (`self.Custom Pan Z`))
    (set `self.WalkedThru` true)
    (`KismetSystemLibrary.Delay` 6.0)
    (set `/Game/Variant_SideScroller/Blueprints/Player/BP_Player.MovementInput` true _asbp_player)))

(fn `UserConstructionScript`)